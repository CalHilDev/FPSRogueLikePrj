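; BP_RandomSpawner periodically spawns BP_EnemyAI at random reachable points around the first-person player, passing the player's difficulty and an XP reward scalable through AlterXP.
; A looping timer calls SpawnEnemy, which recursively spawns a random-sized batch bounded by ExtraSpawnLimit.
; The tick after each batch spawns just one enemy.
; High limits shrink SpawnTime after batches, but the running timer is never reset with the new value.
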(event Custom|SpawnEnemy
  (bind _extraspawnlimit (Variables|Default|GetExtraSpawnLimit))
  (bind _asbp_first_person_character (Utilities|Casting|CastToBP_FirstPersonCharacter (Game|GetPlayerCharacter 0)))
  (Game|SpawnActorfromClass "/Game/Blueprints/BP_EnemyAI.BP_EnemyAI_C" (Math|Transform|MakeTransform (.RandomLocation (AI|Navigation|GetRandomReachablePointinRadius (Transformation|GetActorLocation _asbp_first_person_character) 5e+03 0 0)) (Math|Rotator|MakeRotator 0.0 0.0 (Math|Random|RandomFloatinRange 0.0 3.6e+02)) "1.000000,1.000000,1.000000") "AlwaysSpawn" "MultiplyWithRoot" 0 (Variables|Default|GetExperience) (Variables|/Game/FirstPerson/Blueprints/BP_FirstPersonCharacter.BP_FirstPersonCharacter_C|GetEnemyDifficulty _asbp_first_person_character) 0)
  (Development|PrintString (Utilities|String|ToString(Text) (Utilities|Text|FormatText "Spawned Enemy {current}/{limit}" (+ (Variables|Default|GetExtraSpawns) 1) (Variables|Default|GetExtraSpawnLimit))))
  (if (Variables|Default|GetHasExtraSpawned)
    (Variables|Default|SetHasExtraSpawned false)
    (Variables|Default|SetHasExtraRolled false)
    (else
      (if (Variables|Default|GetHasExtraRolled)
        _
        (else
          (bind _output_get (Variables|Default|SetExtraSpawns (Math|Random|RandomIntegerinRange (Math|Integer|Clamp(Integer) (/ _extraspawnlimit 2) 0 25) (Math|Integer|Clamp(Integer) _extraspawnlimit 0 50))))
          (Variables|Default|SetHasExtraRolled true)))
      (if (> _output_get 0)
        (Math|Integer|DecrementInt (Variables|Default|GetExtraSpawns)
          (:%20%20
            (CallFunction|SpawnEnemy)))
        (else
          (Variables|Default|SetHasExtraSpawned true)
          (Variables|Default|SetExtraSpawns 0)
          (bind _result (Math|Integer|IncrementInt (Variables|Default|GetCurrentSpawnSequence))
            (:%20%20
              (Development|PrintString (Utilities|String|ToString(Text) (Utilities|Text|FormatText "Spawn Sequence {no} Ended" _result)))
              (Variables|Default|SetHasExtraRolled false)
              (if (> (Variables|Default|GetExtraSpawnLimit) 50)
                (Variables|Default|SetSpawnTime (* (Variables|Default|GetSpawnTime) 0.99))))))))))

(event Custom|AlterXP
  (params (Multiplier :type Float%20%28double-precision%29))
  (Variables|Default|SetExperience (* Multiplier (Variables|Default|GetExperience))))

(event EventBeginPlay
  (Utilities|Time|SetTimerbyEvent (delegate Custom|SpawnEnemy) (Variables|Default|GetSpawnTime) true))

(fn ConstructionScript)