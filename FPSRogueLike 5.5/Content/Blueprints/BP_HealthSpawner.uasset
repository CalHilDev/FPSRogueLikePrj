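; BP_HealthSpawner is a spawner actor that periodically drops health pickups around the player.
; On BeginPlay it starts a looping timer at SpawnTime that spawns BP_HealthPickUp at a random reachable navigation point within a large radius of the first-person character.
; SpawnTimeBuff multiplies SpawnTime by a given factor but does not restart the timer, so the running interval stays unchanged.
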(event Custom|SpawnHealth
  (bind _asbp_first_person_character (Utilities|Casting|CastToBP_FirstPersonCharacter (Game|GetPlayerCharacter 0)))
  (Game|SpawnActorfromClass "/Game/Blueprints/BP_HealthPickUp.BP_HealthPickUp_C" (Math|Transform|MakeTransform (.RandomLocation (AI|Navigation|GetRandomReachablePointinRadius (Transformation|GetActorLocation _asbp_first_person_character) 1e+04 0 0)) "0, 0, 0" "1.000000,1.000000,1.000000") "Undefined" "MultiplyWithRoot" 0 0))

(event Custom|SpawnTimeBuff
  (params (SpawnTimeMulti :type Float%20%28double-precision%29))
  (Variables|Default|SetSpawnTime (* SpawnTimeMulti (Variables|Default|GetSpawnTime))))

(event EventBeginPlay
  (Utilities|Time|SetTimerbyEvent (delegate Custom|SpawnHealth) (Variables|Default|GetSpawnTime) true))

(fn ConstructionScript)