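; Hidden, non-ticking audio manager actor that starts default music on BeginPlay and exposes music, ambience and positional SFX playback.
; Music and ambience each swap tracks on one audio component with back-to-back fade calls, without waiting.
; Per-category volumes save to an AudioSettings slot and load at startup, falling back to a default.
; SFX playback bypasses its component's volume multiplier, and PlayDialogue is an empty stub.
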(event EventBeginPlay
  (Actor|SetLifeSpan 0.0)
  (Rendering|SetActorHiddenInGame true)
  (Actor|Tick|SetActorTickEnabled false)
  (CallFunction|LoadAudioSettings)
  (CallFunction|PlayMusic (Variables|Default|GetDefaultMusic)))

(fn ConstructionScript)

(fn PlayMusic
  (params (NewTrack :type Sound%20Base%20Object%20Reference))
  (bind _musicaudio (Variables|Default|GetMusicAudio))
  (Audio|Components|Audio|FadeOut _musicaudio 1.0 0.0 "Linear" :!class /Script/Engine.AudioComponent)
  (Audio|Components|Audio|SetSound _musicaudio NewTrack)
  (Audio|Components|Audio|FadeIn (Variables|Default|GetMusicAudio) 1.0 1.0 0.0 "Linear" :!class /Script/Engine.AudioComponent)
  (Audio|Components|Audio|Play (Variables|Default|GetMusicAudio) 0.0))

(fn PlaySFX
  (params (NewSFX :type Sound%20Base%20Object%20Reference) (SFXLocation :type Vector))
  (Audio|PlaySoundatLocation NewSFX SFXLocation "0, 0, 0" 1.0 1.0 0.0 0 0 0 0))

(fn PlayAmbience
  (params (NewAmbience :type Sound%20Base%20Object%20Reference))
  (bind _ambienceaudio (Variables|Default|GetAmbienceAudio))
  (Audio|Components|Audio|FadeOut _ambienceaudio 1.0 0.0 "Linear" :!class /Script/Engine.AudioComponent)
  (Audio|Components|Audio|SetSound _ambienceaudio NewAmbience)
  (Audio|Components|Audio|FadeIn (Variables|Default|GetAmbienceAudio) 1.0 1.0 0.0 "Linear" :!class /Script/Engine.AudioComponent)
  (Audio|Components|Audio|Play (Variables|Default|GetAmbienceAudio) 0.0))

(fn PlayDialogue
  (params (NewDialogue :type Sound%20Base%20Object%20Reference)))

(fn SaveAudioSettings
  (bind _returnvalue (SaveGame|CreateSaveGameObject "/Game/Blueprints/BP_SaveAudioSettings.BP_SaveAudioSettings_C"))
  (bind _output_get (Variables|Default|SetSaveRef _returnvalue))
  (Variables|/Game/Blueprints/BP_SaveAudioSettings.BP_SaveAudioSettings_C|SetMusicVolume _output_get (Variables|Default|GetMusicVolume))
  (Variables|/Game/Blueprints/BP_SaveAudioSettings.BP_SaveAudioSettings_C|SetSFXVolume _output_get (Variables|Default|GetSFXVolume))
  (Variables|/Game/Blueprints/BP_SaveAudioSettings.BP_SaveAudioSettings_C|SetDialogueVolume _output_get (Variables|Default|GetDialogueVolume))
  (Variables|/Game/Blueprints/BP_SaveAudioSettings.BP_SaveAudioSettings_C|SetAmbienceVolume _output_get (Variables|Default|GetAmbienceVolume))
  (SaveGame|SaveGametoSlot (Variables|Default|GetSaveRef) "AudioSettings"))

(fn LoadAudioSettings
  (bind _defaultvolume (Variables|Default|GetDefaultVolume))
  (bind _returnvalue (SaveGame|DoesSaveGameExist "AudioSettings"))
  (if _returnvalue
    (bind _returnvalue_2 (SaveGame|LoadGamefromSlot "AudioSettings"))
    (bind _asbp_save_audio_settings (Utilities|Casting|CastToBP_SaveAudioSettings _returnvalue_2))
    (bind _output_get (Variables|Default|SetLoadedSettings _asbp_save_audio_settings))
    (bind _output_get_2 (Variables|Default|SetMusicVolume (Variables|/Game/Blueprints/BP_SaveAudioSettings.BP_SaveAudioSettings_C|GetMusicVolume _output_get)))
    (Audio|Components|Audio|SetVolumeMultiplier (Variables|Default|GetMusicAudio) _output_get_2 :!class /Script/Engine.AudioComponent)
    (bind _output_get_3 (Variables|Default|SetSFXVolume (Variables|/Game/Blueprints/BP_SaveAudioSettings.BP_SaveAudioSettings_C|GetSFXVolume _output_get)))
    (Audio|Components|Audio|SetVolumeMultiplier (Variables|Default|GetSFXAudio) _output_get_3 :!class /Script/Engine.AudioComponent)
    (bind _output_get_4 (Variables|Default|SetDialogueVolume (Variables|/Game/Blueprints/BP_SaveAudioSettings.BP_SaveAudioSettings_C|GetDialogueVolume _output_get)))
    (Audio|Components|Audio|SetVolumeMultiplier (Variables|Default|GetDialogueAudio) _output_get_4 :!class /Script/Engine.AudioComponent)
    (bind _output_get_5 (Variables|Default|SetAmbienceVolume (Variables|/Game/Blueprints/BP_SaveAudioSettings.BP_SaveAudioSettings_C|GetAmbienceVolume _output_get)))
    (Audio|Components|Audio|SetVolumeMultiplier (Variables|Default|GetAmbienceAudio) _output_get_5 :!class /Script/Engine.AudioComponent)
    (else
      (bind _output_get_6 (Variables|Default|SetMusicVolume _defaultvolume))
      (Audio|Components|Audio|SetVolumeMultiplier (Variables|Default|GetMusicAudio) _output_get_6 :!class /Script/Engine.AudioComponent)
      (bind _output_get_7 (Variables|Default|SetSFXVolume _defaultvolume))
      (Audio|Components|Audio|SetVolumeMultiplier (Variables|Default|GetSFXAudio) _output_get_7 :!class /Script/Engine.AudioComponent)
      (bind _output_get_8 (Variables|Default|SetDialogueVolume _defaultvolume))
      (Audio|Components|Audio|SetVolumeMultiplier (Variables|Default|GetDialogueAudio) _output_get_8 :!class /Script/Engine.AudioComponent)
      (bind _output_get_9 (Variables|Default|SetAmbienceVolume _defaultvolume))
      (Audio|Components|Audio|SetVolumeMultiplier (Variables|Default|GetAmbienceAudio) _output_get_9 :!class /Script/Engine.AudioComponent))))