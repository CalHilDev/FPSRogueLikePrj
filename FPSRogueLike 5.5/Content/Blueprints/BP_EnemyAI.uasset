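; Orc enemy character that roams, chases and melees the player, with Difficulty scaling health, damage and speed.
; Pawn sensing starts looping line-trace sight checks that switch between chase and roam, while a despawn timer resets on engagement.
; Weapon-fed powerup variables drive bleed, slow/frostbite, cauterise, lifesteal and stacking combustion that explodes on death.
; Tick updates the billboarded health bar and triggers death, awarding XP, kills and score to the player.
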(event OnSeePawn(PawnSensing)
  (params (Pawn :type Pawn%20Object%20Reference))
  ;[1 1 1] Enable Chase State
  (Variables|Default|SetSeenPawn Pawn)
  (Utilities|Time|ClearandInvalidateTimerbyHandle (Variables|Default|GetLostSightTimerHandle))
  (CallFunction|LineOfSight))

(event Custom|FollowPlayer
  ;[1 1 1] Chase & Attack
  (Utilities|Time|ClearandInvalidateTimerbyHandle (Variables|Default|GetRoamTimerHandle))
  (if (Variables|Default|GethasFollowSoundPlayed)
    _
    (else
      (Audio|PlaySoundatLocation "/Game/Audio/OrcChase.OrcChase" (Transformation|GetWorldLocation (Variables|Collision|GetCapsuleComponent)) "0, 0, 0" 1.0 1.0 0.0 0 0 0 0)
      (Variables|Default|SethasFollowSoundPlayed true)))
  (Variables|Default|SetisRoaming false)
  (CallFunction|ResetDespawnTimer)
  (if (Variables|Default|GetisSeeingPlayer)
    (AI|AIMoveTo self "0, 0, 0" (Game|GetPlayerCharacter 0) 5.0 false
      (:OnSuccess
        (if (Variables|Default|GetcanAttack)
          (Variables|Default|SetcanAttack false)
          (bind _returnvalue (Animation|PlayAnimMontage "/Game/Animations/EnemyAI/AM_OrcAttack.AM_OrcAttack" 2.0 "None"))
          (Game|Damage|ApplyDamage (Game|GetPlayerCharacter 0) (Variables|Default|Getdamage) 0 self)
          (Utilities|Time|SetTimerbyEvent (delegate Custom|ResetCanAttack) _returnvalue)
          (CallFunction|ResetDespawnTimer))))
    (else
      (CallFunction|RandomRoam))))

(event Custom|DespawnEnemy
  ;[1 1 1] Start
  (Actor|DestroyActor)
  (Utilities|Time|ClearandInvalidateTimerbyHandle (Variables|Default|GetRoamTimerHandle)))

(event Custom|BleedCheck
  (params (bleedCheck :type Boolean))
  ;[1 1 1] Bleeding
  (bind _output_get (Variables|Default|SetisBleeding bleedCheck))
  (if _output_get
    (CallFunction|Bleeding)))

(event Custom|SetBleedDamage
  (params (WeaponDamage :type Float%20%28double-precision%29))
  ;[1 1 1] Bleeding
  (bind _asbp_first_person_character (Utilities|Casting|CastToBP_FirstPersonCharacter (Game|GetPlayerCharacter 0)))
  (Variables|Default|SetbleedDuration (Variables|/Game/FirstPerson/Blueprints/BP_Weapon_Component.BP_Weapon_Component_C|GetBleedDuration (Variables|/Game/FirstPerson/Blueprints/BP_FirstPersonCharacter.BP_FirstPersonCharacter_C|GetBP_Weapon_Component _asbp_first_person_character)))
  (Variables|Default|SetbleedDamage (* (/ (* (* WeaponDamage 0.5) (Variables|/Game/FirstPerson/Blueprints/BP_Weapon_Component.BP_Weapon_Component_C|GetBleedMultiplier (Variables|/Game/FirstPerson/Blueprints/BP_FirstPersonCharacter.BP_FirstPersonCharacter_C|GetBP_Weapon_Component _asbp_first_person_character))) (Variables|Default|GetinitialBleedDuration)) (Variables|Default|GetbleedDuration))))

(event Custom|ApplyBleed
  (bind _bleeddamage (Variables|Default|GetbleedDamage))
  (bind _bleedduration (Variables|Default|GetbleedDuration))
  (bind _bleedchancetoslow (Variables|Default|GetbleedChanceToSlow))
  (bind _returnvalue (/ _bleeddamage _bleedduration))
  ;[1 1 1] Bleeding
  (if (> _bleedchancetoslow 0.0)
    (if (< _bleedchancetoslow (Math|Random|RandomFloatinRange 1.0 1e+02))
      (CallFunction|MoveSpeedDebuff (Variables|Default|GetslowLimit) (Variables|Default|GetslowPotency))))
  (Utilities|Casting|CastToBP_FirstPersonCharacter (Game|GetPlayerCharacter 0))
  (Variables|Default|Sethealth (- (Variables|Default|Gethealth) _returnvalue))
  (CallFunction|ShowDamageNumber _returnvalue false)
  (Variables|Default|SetbleedDamageAccumulated (+ _returnvalue (Variables|Default|GetbleedDamageAccumulated)))
  (if (>= (Variables|Default|GetbleedDamageAccumulated) (Variables|Default|GetbleedDamage))
    (CallFunction|FinishBleed)))

(event Custom|Bleeding
  ;[1 1 1] Bleeding
  (Rendering|Material|SetScalarParameterValue (Variables|Default|GetEnemyMat) "BleedIntensity" 0.5 :!class /Script/Engine.MaterialInstanceDynamic)
  (bind _returnvalue (Utilities|Time|SetTimerbyEvent (delegate Custom|ApplyBleed) 1.0 true))
  (Variables|Default|SetdamageTimer _returnvalue))

(event Custom|TriggerCombustion
  (bind _returnvalue (Transformation|GetActorLocation))
  (bind _combustionradius (Variables|Default|GetcombustionRadius))
  ;[0.15 0.15 0.15 0.5] Combustion
  (bind _output_get (Variables|Default|SetcombustionDamage (* (Variables|Default|GetcombustionBaseDamage) (Variables|Default|GetcombustStacks))))
  (Game|Damage|ApplyRadialDamage _output_get _returnvalue _combustionradius "/Game/Blueprints/BP_DamageTypeCombustion.BP_DamageTypeCombustion_C" (Utilities|Array|MakeArray (Game|GetPlayerCharacter 0) self) 0 0 true "ECC_Visibility")
  (bind _returnvalue_2 (Niagara|SpawnSystematLocation "/Game/Niagara/NS_Explosion.NS_Explosion" _returnvalue))
  (Niagara|SetNiagaraVariable(Float) _returnvalue_2 "ExplosionRadius" _combustionradius)
  (Audio|PlaySoundatLocation "/Game/Audio/Combustion.Combustion" _returnvalue "0, 0, 0" 1.0 1.0 0.0 0 0 0 0)
  (Variables|Default|SetcombustStacks 0))

(event Custom|ApplyCombustStacks
  (params (StacksToAdd :type Integer))
  ;[0.15 0.15 0.15 0.5] Combustion stack incrementation
  (Variables|Default|SetcombustStacks (Math|Integer|Clamp(Integer) (+ (Variables|Default|GetcombustStacks) StacksToAdd) 0 (Variables|Default|GetmaxCombustStacks))))

(event Custom|Death
  ;[1 1 1] Enemy Death
  (Utilities|Time|ClearandInvalidateTimerbyHandle (Variables|Default|GetRoamTimerHandle))
  (Audio|PlaySoundatLocation "/Game/Audio/OrcDeath.OrcDeath" (Transformation|GetWorldLocation (Variables|Collision|GetCapsuleComponent self)) "0, 0, 0" 1.0 1.0 0.0 0 0 0 0)
  (if (> (Variables|Default|GetcombustStacks) 0)
    (CallFunction|TriggerCombustion))
  (Actor|DestroyActor)
  (bind _asbp_first_person_character (Utilities|Casting|CastToBP_FirstPersonCharacter (Game|GetPlayerCharacter 0)))
  (Default|AddXP _asbp_first_person_character (Variables|Default|GetxpGiven))
  (bind _result (Math|Integer|IncrementInt (Variables|/Game/FirstPerson/Blueprints/BP_FirstPersonCharacter.BP_FirstPersonCharacter_C|GetKillCounter _asbp_first_person_character))
    (:%20%20
      (Variables|/Game/FirstPerson/Blueprints/BP_FirstPersonCharacter.BP_FirstPersonCharacter_C|SetKillCounter _asbp_first_person_character _result)
      (bind _output_get (Variables|/Game/FirstPerson/Blueprints/BP_FirstPersonCharacter.BP_FirstPersonCharacter_C|SetScore _asbp_first_person_character (+ (* (Variables|Default|GetscoreAwarded) (+ (/ (Variables|/Game/FirstPerson/Blueprints/BP_FirstPersonCharacter.BP_FirstPersonCharacter_C|GetLevel _asbp_first_person_character) 100) 1.0)) (Variables|/Game/FirstPerson/Blueprints/BP_FirstPersonCharacter.BP_FirstPersonCharacter_C|GetScore _asbp_first_person_character))))
      (bind _asbp_game_instance (Utilities|Casting|CastToBP_GameInstance (Game|GetGameInstance)))
      (bind _output_get_2 (Variables|/Game/Blueprints/BP_GameInstance.BP_GameInstance_C|SetCurrentScore _asbp_game_instance _output_get))
      (Development|PrintString (Utilities|String|ToString(Float) _output_get_2))
      (if (> (Variables|/Game/FirstPerson/Blueprints/BP_Weapon_Component.BP_Weapon_Component_C|GetMomentumDamage (Variables|/Game/FirstPerson/Blueprints/BP_FirstPersonCharacter.BP_FirstPersonCharacter_C|GetBP_Weapon_Component _asbp_first_person_character)) 0.0)
        (Variables|/Game/FirstPerson/Blueprints/BP_Weapon_Component.BP_Weapon_Component_C|SetHasKilledRecently (Variables|/Game/FirstPerson/Blueprints/BP_FirstPersonCharacter.BP_FirstPersonCharacter_C|GetBP_Weapon_Component _asbp_first_person_character) true)))))

(event Custom|UpdateCombustionVariables
  (params (combustionDamage :type Float%20%28double-precision%29) (combustionStackLimit :type Integer) (combustionRadius :type Float%20%28double-precision%29) (canCauterise :type Boolean) (cauteriseMultiplier :type Float%20%28double-precision%29))
  ;[0.15 0.15 0.15 0.5] Combustion Variables
  (Variables|Default|SetcombustionBaseDamage combustionDamage)
  (Variables|Default|SetmaxCombustStacks combustionStackLimit)
  (Variables|Default|SetcombustionRadius combustionRadius)
  (Variables|Default|SetcanCauterise canCauterise)
  (Variables|Default|SetcauteriseMultiplier cauteriseMultiplier))

(event Custom|UpdateFrostbite
  (params (FrostbiteActive :type Boolean) (FrostbiteModifier :type Float%20%28double-precision%29))
  ;[0.15 0.15 0.15 0.5] Updates Frostbite Variables (when slow aura triggers)
  (Variables|Default|SetisFrostbite FrostbiteActive)
  (Variables|Default|SetfrostbiteModifier FrostbiteModifier))

(event Custom|LifestealCheck
  ;[0.15 0.15 0.15 0.5] Calls Lifesteal IF Enabled
  (if (Variables|Default|GetisLifesteal)
    (if (== (Variables|Default|Gethealth) (Variables|Default|GetmaxHealth))
      (bind _asbp_first_person_character (Utilities|Casting|CastToBP_FirstPersonCharacter (Game|GetPlayerCharacter 0)))
      (Default|Lifesteal _asbp_first_person_character))))

(event Custom|FinishBleed
  ;[1 1 1] Bleeding
  (Variables|Default|SetbleedDone true)
  (Utilities|Time|ClearandInvalidateTimerbyHandle (Variables|Default|GetdamageTimer))
  (Variables|Default|SetisBleeding false)
  (Variables|Default|SetbleedDone false)
  (Variables|Default|SetbleedDamageAccumulated 0.0)
  (Rendering|Material|SetScalarParameterValue (Variables|Default|GetEnemyMat) "BleedIntensity" 0.0 :!class /Script/Engine.MaterialInstanceDynamic))

(event Custom|UpdatePowerupVariablesFromWeapon
  (params (BleedChanceToSlow :type Float%20%28double-precision%29) (IsLifesteal :type Boolean) (GunDamage :type Float%20%28double-precision%29))
  ;[0.15 0.15 0.15 0.5] Reads powerup bools from weapon
  (Variables|Default|SetbleedChanceToSlow BleedChanceToSlow)
  (Variables|Default|SetisLifesteal IsLifesteal)
  (Variables|Default|SetGun%20Damage GunDamage))

(event Custom|AlterXPGiven
  (params (XPGiven :type Float%20%28double-precision%29))
  ;[1 1 1] Start
  (Variables|Default|SetxpGiven XPGiven))

(event Custom|AlterDifficulty
  (params (difficulty :type Float%20%28double-precision%29))
  ;[1 1 1] Start
  (Variables|Default|Setdifficulty difficulty))

(event Custom|RemoveSlow
  ;[1 1 1] Slow (from freezing)
  (if (> (Variables|Default|GetslowStacks) 0)
    (bind _result (Math|Integer|DecrementInt (Variables|Default|GetslowStacks))
      (:%20%20
        (if (<= _result 0)
          (Rendering|Material|SetScalarParameterValue (Variables|Default|GetEnemyMat) "SlowIntensity" 0.0 :!class /Script/Engine.MaterialInstanceDynamic)
          (CallFunction|Debug (Utilities|String|ToString(Text) (Utilities|Text|FormatText "Slow Stacks after removal: {Slow Stacks}" (Variables|Default|GetslowStacks)))))))
    (else
      (Utilities|Time|ClearandInvalidateTimerbyHandle (Variables|Default|GetSlowRemovalTimerHandle)))))

(event Custom|ResetCanAttack
  (Variables|Default|SetcanAttack true)
  (CallFunction|FollowPlayer))

(event Custom|Debug
  (params (DebugText :type String))
  (Development|PrintString (Utilities|String|ToString(Text) (Utilities|Text|FormatText "{Debug} {Enemy}" DebugText (Utilities|GetDisplayName self)))))

(event Custom|LoSCheck
  (bind _seenpawn (Variables|Default|GetSeenPawn))
  (if (Utilities|IsValid _seenpawn)
    (bind _outhit (Collision|LineTraceByChannel (Transformation|GetActorLocation self) (Transformation|GetActorLocation _seenpawn) "TraceTypeQuery1" false 0 "None"))
    (if (== (.HitActor (Collision|BreakHitResult _outhit)) _seenpawn)
      (Utilities|Time|ClearandInvalidateTimerbyHandle (Variables|Default|GetLostSightTimerHandle))
      (Variables|Default|SetisSeeingPlayer true)
      (CallFunction|FollowPlayer)
      (else
        (bind _returnvalue (Utilities|Time|SetTimerbyEvent (delegate Custom|NotInLoS) 1.0))
        (Variables|Default|SetLostSightTimerHandle _returnvalue)))
    (else
      (Utilities|Time|ClearandInvalidateTimerbyHandle (Variables|Default|GetCheckSightTimerHandle))
      (CallFunction|Debug "LoS Validation Fail"))))

(event Custom|LineOfSight
  (bind _returnvalue (Utilities|Time|SetTimerbyEvent (delegate Custom|LoSCheck) 0.2 true))
  (Variables|Default|SetCheckSightTimerHandle _returnvalue))

(event Custom|NotInLoS
  (bind _outhit (Collision|LineTraceByChannel (Transformation|GetActorLocation self) (Transformation|GetActorLocation (Variables|Default|GetSeenPawn)) "TraceTypeQuery1" false 0 "None"))
  (if (== (.HitActor (Collision|BreakHitResult _outhit)) (Variables|Default|GetSeenPawn))
    (Variables|Default|SetisSeeingPlayer true)
    (CallFunction|FollowPlayer)
    (else
      (Variables|Default|SetisSeeingPlayer false)
      (CallFunction|RandomRoam))))

(event Custom|Cauterise
  (bind _bleeddamage (Variables|Default|GetbleedDamage))
  (bind _bleeddamageaccumulated (Variables|Default|GetbleedDamageAccumulated))
  (bind _cauterisemultiplier (Variables|Default|GetcauteriseMultiplier))
  (bind _returnvalue (- _bleeddamage _bleeddamageaccumulated))
  (bind _returnvalue_2 (* _returnvalue _cauterisemultiplier))
  ;[0.15 0.15 0.15 0.5] Cauterise mechanic
  (if (Variables|Default|GetisBleeding)
    (Variables|Default|Sethealth (- (Variables|Default|Gethealth) _returnvalue_2))
    (CallFunction|ShowDamageNumber _returnvalue_2 false)
    (CallFunction|FinishBleed)))

(event Custom|ShowDamageNumber
  (params (DamageAmount :type Float%20%28double-precision%29) (IsCrit :type Boolean))
  ;[0.15 0.15 0.15 0.5] Brings the damage number to the screen
  (Game|SpawnActorfromClass "/Game/Blueprints/BP_DamageNumberActor.BP_DamageNumberActor_C" (Math|Conversions|ToTransform(Vector) (+ (Transformation|GetActorLocation) (Math|Vector|MakeVector (Math|Random|RandomFloatinRange -2e+01 2e+01) (Math|Random|RandomFloatinRange -2e+01 2e+01) 8e+01))) "Undefined" "MultiplyWithRoot" 0 DamageAmount IsCrit 0))

(event Custom|SetMaxMoveSpeed
  ;[0.15 0.15 0.15 0.5] Change movement speed based on enemy difficulty
  (if (> (Variables|Default|GetmaxMoveSpeed) 7.5e+02)
    (Variables|Default|SetmaxMoveSpeed 7.5e+02)
    (else
      (Variables|Default|SetmaxMoveSpeed (* (Variables|Default|GetmaxMoveSpeed) (+ (/ (- (Variables|Default|Getdifficulty) 1.0) 8.0) 1.0))))))

(event Custom|MoveSpeedDebuff
  (params (StackLimit :type Integer) (SlowPotency :type Float%20%28double-precision%29))
  ;[1 1 1] Slow (from freezing)
  (Variables|Default|SetslowLimit StackLimit)
  (Variables|Default|SetslowPotency SlowPotency)
  (if (< (Variables|Default|GetslowStacks) (Variables|Default|GetslowLimit))
    (Math|Integer|IncrementInt (Variables|Default|GetslowStacks)
      (:%20%20
        (Rendering|Material|SetScalarParameterValue (Variables|Default|GetEnemyMat) "SlowIntensity" 0.5 :!class /Script/Engine.MaterialInstanceDynamic)
        (bind _output_get (Variables|/Script/Engine.CharacterMovementComponent|SetMaxWalkSpeed (Variables|Character|GetCharacterMovement) (- (Variables|Default|GetmaxMoveSpeed) (* (Variables|Default|GetslowStacks) (Variables|Default|GetslowPotency)))))
        (if (Variables|Default|GetisFrostbite)
          (bind _returnvalue (Game|Damage|ApplyDamage self (* (Variables|Default|GetfrostbiteModifier) (+ (/ (Variables|Default|GetGun%20Damage) 2e+01) 5.0)) 0 0)))
        (bind _returnvalue_2 (Utilities|Time|SetTimerbyEvent (delegate Custom|RemoveSlow) (Variables|Default|GetchillDuration) true))
        (Variables|Default|SetSlowRemovalTimerHandle _returnvalue_2)))))

(event Custom|RoamAgain
  (if (not (Variables|Default|GetisSeeingPlayer))
    (Variables|Default|SetroamCheck false)
    (CallFunction|RandomRoam)))

(event Custom|RandomRoam
  ;[1 1 1] Roaming
  (if (not (Variables|Default|GetroamCheck))
    (Variables|Default|SetisRoaming true)
    (AI|AIMoveTo self (.RandomLocation (AI|Navigation|GetRandomReachablePointinRadius (Transformation|GetActorLocation) 1e+03 0 0)) 0 5.0 false
      (:then
        (Variables|Default|SetroamCheck true))
      (:OnSuccess
        (Variables|Default|SetisRoaming false)
        (Utilities|Time|ClearandInvalidateTimerbyHandle (Variables|Default|GetRoamTimerHandle) :!label _label)
        (bind _returnvalue (Utilities|Time|SetTimerbyEvent (delegate Custom|RoamAgain) 1.0))
        (Variables|Default|SetRoamTimerHandle _returnvalue))
      (:OnFail
        (Utilities|FlowControl|Delay 0.2)
        (if (not (Variables|Default|GetisSeeingPlayer))
          (goto _label))))))

(event Custom|ResetDespawnTimer
  ;[1 1 1] Start
  (Utilities|Time|ClearandInvalidateTimerbyHandle (Variables|Default|GetdespawnTimerHandle))
  (bind _returnvalue (Utilities|Time|SetTimerbyEvent (delegate Custom|DespawnEnemy) (Variables|Default|GetdespawnTime)))
  (Variables|Default|SetdespawnTimerHandle _returnvalue))

(event Game|Damage|EventAnyDamage
  (params (Damage :type Float%20%28single-precision%29) (DamageType :type Damage%20Type%20Object%20Reference) (InstigatedBy :type Controller%20Object%20Reference) (DamageCauser :type Actor%20Object%20Reference))
  ;[1 1 1] Take Damage
  (Variables|Default|SetisRoaming false)
  (if (> (Variables|Default|GetHealth) 0.0)
    (if (== (Utilities|GetClass DamageType) "/Game/Blueprints/BP_DamageTypeCombustion.BP_DamageTypeCombustion_C")
      (if (Variables|Default|GetcanCauterise)
        (CallFunction|Cauterise))))
  (CallFunction|LifestealCheck)
  (Variables|Default|SetHealth (- (Variables|Default|GetHealth) Damage))
  (CallFunction|ShowDamageNumber Damage (Variables|Default|GethasCrit))
  (Variables|Default|SethasCrit false)
  (Variables|Default|SetisSeeingPlayer true)
  (CallFunction|ResetDespawnTimer)
  (CallFunction|FollowPlayer))

(event EventTick
  (params (DeltaSeconds :type Float%20%28single-precision%29))
  ;[1 1 1] Update
  ;;[1 1 1] Health Bar
  (bind _aswp_enemy_health_bar (Utilities|Casting|CastToWP_EnemyHealthBar (UserInterface|GetWidget (Variables|Default|GetHealthBarWidget))))
  (Progress|SetPercent (Variables|/Game/UI/WP_EnemyHealthBar.WP_EnemyHealthBar_C|GetHealthBar _aswp_enemy_health_bar) (/ (Variables|Default|Gethealth) (Variables|Default|GetmaxHealth)))
  (Transformation|SetWorldRotation (Variables|Default|GetHealthBarWidget) (Math|Rotator|FindLookatRotation (Transformation|GetWorldLocation (Variables|Default|GetHealthBarWidget)) (Transformation|GetWorldLocation (Variables|/Script/Engine.PlayerCameraManager|GetTransformComponent (Game|GetPlayerCameraManager 0)))) false false)
  (Default|GetStacks _aswp_enemy_health_bar (Variables|Default|GetslowStacks) (Variables|Default|GetcombustStacks))
  (Default|DisplayBleed _aswp_enemy_health_bar (Variables|Default|GetisBleeding))
  (if (Variables|Default|GetisRoaming)
    (Variables|/Script/Engine.CharacterMovementComponent|SetMaxWalkSpeed (Variables|Character|GetCharacterMovement) (/ (Variables|Default|GetmaxMoveSpeed) 4.0))
    (else
      (Variables|/Script/Engine.CharacterMovementComponent|SetMaxWalkSpeed (Variables|Character|GetCharacterMovement) (Variables|Default|GetcurrentMoveSpeed))))
  (if (<= (Variables|Default|Gethealth) 0.0)
    (CallFunction|Death)))

(event EventBeginPlay
  (bind _difficulty (Variables|Default|Getdifficulty))
  ;[1 1 1] Start
  (bind _returnvalue (Utilities|Time|SetTimerbyEvent (delegate Custom|DespawnEnemy) (Variables|Default|GetdespawnTime)))
  (Variables|Default|SetdespawnTimerHandle _returnvalue)
  (Variables|Default|SetmaxHealth (* (Variables|Default|GetmaxHealth) _difficulty))
  (Variables|Default|Setdamage (* (Variables|Default|Getdamage) _difficulty))
  (Variables|Default|Sethealth (Variables|Default|GetmaxHealth))
  (CallFunction|SetMaxMoveSpeed)
  (Variables|Default|SetcurrentMoveSpeed (Variables|Default|GetmaxMoveSpeed))
  (Audio|PlaySoundatLocation "/Game/Audio/OrcSpawn2.OrcSpawn2" (Transformation|GetWorldLocation (Variables|Collision|GetCapsuleComponent)) "0, 0, 0" 1.0 1.0 0.0 0 0 0 0)
  (if (not (Variables|Default|GetisSeeingPlayer))
    (Variables|Default|SethasFollowSoundPlayed false)
    (CallFunction|RandomRoam)
    (bind _returnvalue_2 (Rendering|Material|CreateDynamicMaterialInstance (Variables|Character|GetMesh) 0 "/Game/M_OrcTemp2.M_OrcTemp2" "None" :!class /Script/Engine.PrimitiveComponent))
    (Variables|Default|SetEnemyMat _returnvalue_2)))

(fn ConstructionScript
  (CallFunction|AlterDifficulty (Variables|Default|Getdifficulty))
  (CallFunction|AlterXPGiven (Variables|Default|GetxpGiven)))