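; BP_BuffPickUp is a configurable pickup that grants a timed buff to the player.
; Its construction script sets the pickup mesh from a mesh asset variable.
; On any actor overlap it calls ApplyBuff on player 0's BP_FirstPersonCharacter with its type, amount and duration, then destroys itself, without checking which actor overlapped.
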(event Collision|EventActorBeginOverlap
  (params (OtherActor :type Actor%20Object%20Reference))
  (bind _asbp_first_person_character (Utilities|Casting|CastToBP_FirstPersonCharacter (Game|GetPlayerCharacter 0)))
  (Default|ApplyBuff _asbp_first_person_character (Variables|Default|GetPickupType) (Variables|Default|GetBuffAmount) (Variables|Default|GetDuration))
  (Actor|DestroyActor))

(fn ConstructionScript
  (Components|StaticMesh|SetStaticMesh (Variables|Default|GetPickUpMesh) (Variables|Default|GetPickupMeshAsset)))