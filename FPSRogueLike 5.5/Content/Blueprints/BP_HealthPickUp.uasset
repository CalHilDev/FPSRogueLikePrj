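; BP_HealthPickUp is a health pickup that heals the first-person player character on touch.
; When the collision component overlaps an actor tagged Player, it casts to BP_FirstPersonCharacter, calls IncreaseHealth with HealAmount, plays a 2D sound and destroys itself.
; A HealAmountBuff event raises HealAmount by a fixed step, with no caller in this graph.
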(event OnComponentBeginOverlap(Collission)
  (params (OverlappedComponent :type Primitive%20Component%20Object%20Reference) (OtherActor :type Actor%20Object%20Reference) (OtherComp :type Primitive%20Component%20Object%20Reference) (OtherBodyIndex :type Integer) (bFromSweep :type Boolean) (SweepResult :type Hit%20Result%20Structure%20%28by%20ref%29))
  (if (Actor|ActorHasTag OtherActor "Player")
    (bind _asbp_first_person_character (Utilities|Casting|CastToBP_FirstPersonCharacter OtherActor))
    (Default|IncreaseHealth _asbp_first_person_character (Variables|Default|GetHealAmount))
    (Audio|PlaySound2D "/Game/Audio/HealthPickUp.HealthPickUp" 1.0 1.0 0.0 0 0)
    (Actor|DestroyActor)))

(event Custom|HealAmountBuff
  (Variables|Default|SetHealAmount (+ (Variables|Default|GetHealAmount) 5.0)))

(fn ConstructionScript)