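; BP_DamageNumberActor is a short-lived actor that shows a floating damage number in the world.
; On BeginPlay it passes the damage amount and crit flag to its WB_DamageNumber widget and plays that widget's FadeUp animation.
; A MoveUp timeline lerps the actor upward from its start location, then destroys it when finished.
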(event EventBeginPlay
  (Variables|Default|SetStartLocation (Transformation|GetActorLocation))
  (bind _aswb_damage_number (Utilities|Casting|CastToWB_DamageNumber (UserInterface|GetUserWidgetObject (Variables|Default|GetDamageNumberWidget))))
  (Default|SetDamage _aswb_damage_number (Variables|Default|GetDamageAmount))
  (Default|SetCrit _aswb_damage_number (Variables|Default|GetIsCrit))
  (UserInterface|Animation|PlayAnimation _aswb_damage_number (Variables|/Game/UI/WB_DamageNumber.WB_DamageNumber_C|GetFadeUp _aswb_damage_number) 0.0 1 "Forward" 1.0 false)
  (bind _alpha (Timeline|MoveUp Play)
    (:Update
      (Transformation|SetActorLocation (Math|Vector|Lerp(Vector) (Variables|Default|GetStartLocation) (+ (Variables|Default|GetStartLocation) "0.000000,0.000000,50.000000") _alpha) false false))
    (:Finished
      (Actor|DestroyActor))))

(event Collision|EventActorBeginOverlap
  (params (OtherActor :type Actor%20Object%20Reference)))

(event EventTick
  (params (DeltaSeconds :type Float%20%28single-precision%29)))

(fn ConstructionScript)