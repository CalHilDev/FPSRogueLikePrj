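; SG_Leaderboard holds leaderboard records as parallel arrays of scores, survival times and timestamps.
; SortLeaderboard bubble-sorts an index array by descending score, then uses it to rebuild and replace all three arrays.
; A disabled, unreachable trim attempt would have capped the arrays at MaxArrayEntries.
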(fn SortLeaderboard
  (bind _indexes (Variables|Default|GetIndexes))
  (bind _indexes_2 (Variables|Default|GetIndexes))
  (bind _indexes_3 (Variables|Default|GetIndexes))
  (bind _returnvalue (Utilities|Array|Length _indexes))
  (bind _returnvalue_2 (- _returnvalue 2))
  (Utilities|Array|Clear (Variables|Default|GetIndexes))
  (Utilities|Array|Clear (Variables|Default|GetSortedScores))
  (Utilities|Array|Clear (Variables|Default|GetSortedSurvivalTimes))
  (Utilities|Array|Clear (Variables|Default|GetSortedTimestamps))
  (for _index (range 0 (- (Utilities|Array|Length (Variables|Default|GetScores)) 1))
    (Utilities|Array|Add (Variables|Default|GetIndexes) _index))
  (for _index_2 (range 0 _returnvalue_2)
    (for _index_3 (range 0 (- _returnvalue_2 _index_2))
      (Variables|Default|SetTempIndex (Utilities|Array|Get(acopy) (Variables|Default|GetIndexes) _index_3))
      (if (< (Utilities|Array|Get(acopy) (Variables|Default|GetScores) (Utilities|Array|Get(acopy) (Variables|Default|GetIndexes) _index_3)) (Utilities|Array|Get(acopy) (Variables|Default|GetScores) (Utilities|Array|Get(acopy) (Variables|Default|GetIndexes) (+ _index_3 1))))
        (Utilities|Array|SetArrayElem _indexes_2 _index_3 (Utilities|Array|Get(acopy) (Variables|Default|GetIndexes) (+ _index_3 1)))
        (Utilities|Array|SetArrayElem _indexes_2 (+ _index_3 1) (Variables|Default|GetTempIndex)))))
  (for (_ _array_index) _indexes_3
    (Utilities|Array|Add (Variables|Default|GetSortedScores) (Utilities|Array|Get(acopy) (Variables|Default|GetScores) (Utilities|Array|Get(acopy) _indexes_3 _array_index)))
    (Utilities|Array|Add (Variables|Default|GetSortedSurvivalTimes) (Utilities|Array|Get(acopy) (Variables|Default|GetSurvivalTimes) (Utilities|Array|Get(acopy) _indexes_3 _array_index)))
    (Utilities|Array|Add (Variables|Default|GetSortedTimestamps) (Utilities|Array|Get(acopy) (Variables|Default|GetTimestamps) (Utilities|Array|Get(acopy) _indexes_3 _array_index))))
  (Variables|Default|SetScores (Variables|Default|GetSortedScores))
  (Variables|Default|SetSurvivalTimes (Variables|Default|GetSortedSurvivalTimes))
  (Variables|Default|SetTimestamps (Variables|Default|GetSortedTimestamps)))