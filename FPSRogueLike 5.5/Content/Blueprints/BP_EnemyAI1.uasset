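; Enemy AI character that roams randomly, chases the player on sight or when hit, attacks on reaching them, and awards XP on death.
; Difficulty scales health and damage, while Tick updates movement speed and a camera-facing health bar with status indicators.
; Player weapon stats drive timer-based bleed and burn sharing one timer handle.
; Chill stacks slow it, burning boosts speed, and burn ticks shatter fully chilled enemies when enabled.
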(event OnSeePawn(PawnSensing)
  (params (Pawn :type Pawn%20Object%20Reference))
  ;[1 1 1] Enable Chase State
  (Variables|Default|SetisSeeingPlayer true)
  (CallFunction|FollowPlayer))

(event Custom|FollowPlayer
  ;[1 1 1] Chase & Attack
  (Components|Animation|PlayAnimation (Variables|Character|GetMesh) "/Game/Animations/OrcRunAnimProto7_Anim.OrcRunAnimProto7_Anim" false)
  (Variables|Default|SetisRoaming false)
  (Variables|Default|SetcanAttack true)
  (if (Variables|Default|GetisSeeingPlayer)
    (AI|AIMoveTo self "0, 0, 0" (Game|GetPlayerCharacter 0) 5.0 false
      (:OnSuccess
        (if (Variables|Default|GetcanAttack)
          (Variables|Default|SetcanAttack false)
          (bind _returnvalue (Animation|PlayAnimMontage "/Game/Animations/EnemyAI/AM_EnemyAttack.AM_EnemyAttack" 1.0 "None"))
          (Game|Damage|ApplyDamage (Game|GetPlayerCharacter 0) (Variables|Default|Getdamage) 0 0)
          (Utilities|FlowControl|Delay _returnvalue)
          (CallFunction|RandomRoam))))
    (else
      (Variables|Default|SetisSeeingPlayer false))))

(event Custom|BleedCheck
  (params (bleedCheck :type Boolean))
  ;[1 1 1] Bleeding
  (bind _output_get (Variables|Default|SetisBleeding bleedCheck))
  (if _output_get
    (CallFunction|Bleeding)))

(event Custom|SetBleedDamage
  (params (WeaponDamage :type Float%20%28double-precision%29))
  ;[1 1 1] Bleeding
  (bind _asbp_first_person_character (Utilities|Casting|CastToBP_FirstPersonCharacter (Game|GetPlayerCharacter 0)))
  (Variables|Default|SetbleedDuration (Variables|/Game/FirstPerson/Blueprints/BP_Weapon_Component.BP_Weapon_Component_C|GetBleedDuration (Variables|/Game/FirstPerson/Blueprints/BP_FirstPersonCharacter.BP_FirstPersonCharacter_C|GetBP_Weapon_Component _asbp_first_person_character)))
  (Variables|Default|SetbleedDamage (* (/ (* (* WeaponDamage 0.2) (Variables|/Game/FirstPerson/Blueprints/BP_Weapon_Component.BP_Weapon_Component_C|GetBleedMultiplier (Variables|/Game/FirstPerson/Blueprints/BP_FirstPersonCharacter.BP_FirstPersonCharacter_C|GetBP_Weapon_Component _asbp_first_person_character))) (Variables|Default|GetinitialBleedDuration)) (Variables|Default|GetbleedDuration))))

(event Custom|ApplyBleed
  (bind _bleeddamage (Variables|Default|GetbleedDamage))
  (bind _bleedduration (Variables|Default|GetbleedDuration))
  (bind _returnvalue (/ _bleeddamage _bleedduration))
  ;[1 1 1] Bleeding
  (Variables|Default|Sethealth (- (Variables|Default|Gethealth) _returnvalue))
  (Variables|Default|SetbleedDamageAccumulated (+ _returnvalue (Variables|Default|GetbleedDamageAccumulated)))
  (bind _output_get (Variables|Default|SetbleedDone (>= (Variables|Default|GetbleedDamageAccumulated) (Variables|Default|GetbleedDamage))))
  (if _output_get
    (Utilities|Time|ClearandInvalidateTimerbyHandle (Variables|Default|GetdamageTimer))
    (Variables|Default|SetisBleeding false)
    (Variables|Default|SetbleedDone false)
    (Variables|Default|SetbleedDamageAccumulated 0.0)))

(event Custom|Bleeding
  ;[1 1 1] Bleeding
  (bind _returnvalue (Utilities|Time|SetTimerbyEvent (delegate Custom|ApplyBleed) 1.0 true))
  (Variables|Default|SetdamageTimer _returnvalue))

(event Custom|Death
  ;[1 1 1] Enemy Death
  (Actor|DestroyActor)
  (bind _asbp_first_person_character (Utilities|Casting|CastToBP_FirstPersonCharacter (Game|GetPlayerCharacter 0)))
  (Default|AddXP _asbp_first_person_character (Variables|Default|GetxpGiven))
  (bind _result (Math|Integer|IncrementInt (Variables|/Game/FirstPerson/Blueprints/BP_FirstPersonCharacter.BP_FirstPersonCharacter_C|GetKillCounter _asbp_first_person_character))
    (:%20%20
      (Variables|/Game/FirstPerson/Blueprints/BP_FirstPersonCharacter.BP_FirstPersonCharacter_C|SetKillCounter _asbp_first_person_character _result))))

(event Custom|ShatterCheck
  ;[1 1 1] Shatter Check
  (if (>= (Variables|Default|GetslowStacks) (Variables|Default|GetslowLimit))
    (Variables|Default|SetcanShatter true)
    (else
      (Variables|Default|SetcanShatter false))))

(event Custom|BurnCheck
  (params (burnCheck :type Boolean))
  ;[1 1 1] Burning
  (bind _output_get (Variables|Default|SetisBurning burnCheck))
  (if _output_get
    (CallFunction|Burning)))

(event Custom|AlterXPGiven
  (params (XPGiven :type Float%20%28double-precision%29))
  (Variables|Default|SetxpGiven XPGiven))

(event Custom|AlterDifficulty
  (params (difficulty :type Float%20%28double-precision%29))
  (Variables|Default|Setdifficulty difficulty))

(event Custom|SetBurnDamage
  (params (WeaponDamage :type Float%20%28double-precision%29))
  ;[1 1 1] Burning
  (bind _asbp_first_person_character (Utilities|Casting|CastToBP_FirstPersonCharacter (Game|GetPlayerCharacter 0)))
  (Variables|Default|SetburnDuration (Variables|/Game/FirstPerson/Blueprints/BP_Weapon_Component.BP_Weapon_Component_C|GetBurnDuration (Variables|/Game/FirstPerson/Blueprints/BP_FirstPersonCharacter.BP_FirstPersonCharacter_C|GetBP_Weapon_Component _asbp_first_person_character)))
  (Variables|Default|SetburnDamage (* (/ (* (* WeaponDamage 0.5) (Variables|/Game/FirstPerson/Blueprints/BP_Weapon_Component.BP_Weapon_Component_C|GetBurnMultiplier (Variables|/Game/FirstPerson/Blueprints/BP_FirstPersonCharacter.BP_FirstPersonCharacter_C|GetBP_Weapon_Component _asbp_first_person_character))) (Variables|Default|GetinitialBurnDuration)) (Variables|Default|GetburnDuration))))

(event Custom|ApplyBurn
  (bind _burndamage (Variables|Default|GetburnDamage))
  (bind _burnduration (Variables|Default|GetburnDuration))
  (bind _returnvalue (/ _burndamage _burnduration))
  ;[1 1 1] Burning
  (if (Variables|Default|GetcanShatter)
    (CallFunction|Shatter))
  (Variables|Default|Sethealth (- (Variables|Default|Gethealth) _returnvalue))
  (Variables|Default|SetburnDamageAccumulated (+ _returnvalue (Variables|Default|GetburnDamageAccumulated)))
  (bind _output_get (Variables|Default|SetburnDone (>= (Variables|Default|GetburnDamageAccumulated) (Variables|Default|GetburnDamage))))
  (if _output_get
    (Utilities|Time|ClearandInvalidateTimerbyHandle (Variables|Default|GetdamageTimer))
    (Variables|Default|SetisBurning false)
    (Variables|Default|SetburnDone false)
    (Variables|Default|SetburnDamageAccumulated 0.0)))

(event Custom|Burning
  ;[1 1 1] Burning
  (bind _returnvalue (Utilities|Time|SetTimerbyEvent (delegate Custom|ApplyBurn) 1.0 true))
  (Variables|Default|SetdamageTimer _returnvalue))

(event Custom|MoveSpeedDebuff
  (params (StackLimit :type Integer) (SlowPotency :type Float%20%28double-precision%29))
  ;[1 1 1] Slow (from freezing)
  (Variables|Default|SetslowLimit StackLimit)
  (Variables|Default|SetslowPotency SlowPotency)
  (if (not (Variables|Default|GetisBurning))
    (if (< (Variables|Default|GetslowStacks) (Variables|Default|GetslowLimit))
      (Math|Integer|IncrementInt (Variables|Default|GetslowStacks)
        (:%20%20
          (Variables|/Script/Engine.CharacterMovementComponent|SetMaxWalkSpeed (Variables|Character|GetCharacterMovement) (- (Variables|Default|GetmaxMoveSpeed) (* (Variables|Default|GetslowStacks) (Variables|Default|GetslowPotency))))
          (Utilities|FlowControl|Delay (Variables|Default|GetchillDuration)) ; Duration of MS decrease
          (Math|Integer|DecrementInt (Variables|Default|GetslowStacks)))))))

(event Custom|MoveSpeedBuff
  ;[1 1 1] Speed Boost (from burning)
  (Variables|Default|SetslowStacks 0)
  (Variables|Default|SetcurrentMoveSpeed (* (Variables|Default|GetmaxMoveSpeed) 1.3))
  (Utilities|FlowControl|Delay 5.0) ; Duration of MS increase
  (Variables|Default|SetcurrentMoveSpeed (Variables|Default|GetmaxMoveSpeed)))

(event Custom|RandomRoam
  ;[1 1 1] Roaming
  (Variables|Default|SetisRoaming true)
  (AI|AIMoveTo self (.RandomLocation (AI|Navigation|GetRandomReachablePointinRadius (Transformation|GetActorLocation) 1e+03 0 0)) 0 5.0 false
    (:OnSuccess
      (Utilities|FlowControl|Delay 1.0)
      (Variables|Default|SetisRoaming false)
      (CallFunction|RandomRoam))))

(event Custom|Shatter
  ;[1 1 1] Shatter
  (Variables|Default|SetslowStacks 0)
  (bind _asbp_first_person_character (Utilities|Casting|CastToBP_FirstPersonCharacter (Game|GetPlayerCharacter 0)))
  (Variables|Default|Sethealth (- (Variables|Default|Gethealth) (* (Variables|/Game/FirstPerson/Blueprints/BP_Weapon_Component.BP_Weapon_Component_C|GetShatterMultiplier (Variables|/Game/FirstPerson/Blueprints/BP_FirstPersonCharacter.BP_FirstPersonCharacter_C|GetBP_Weapon_Component _asbp_first_person_character)) (Variables|/Game/FirstPerson/Blueprints/BP_Weapon_Component.BP_Weapon_Component_C|GetGunDamage (Variables|/Game/FirstPerson/Blueprints/BP_FirstPersonCharacter.BP_FirstPersonCharacter_C|GetBP_Weapon_Component _asbp_first_person_character))))))

(event Game|Damage|EventAnyDamage
  (params (Damage :type Float%20%28single-precision%29) (DamageType :type Damage%20Type%20Object%20Reference) (InstigatedBy :type Controller%20Object%20Reference) (DamageCauser :type Actor%20Object%20Reference))
  ;[1 1 1] Take Damage
  (bind _asbp_first_person_character (Utilities|Casting|CastToBP_FirstPersonCharacter (Game|GetPlayerCharacter 0)))
  (if (Variables|/Game/FirstPerson/Blueprints/BP_Weapon_Component.BP_Weapon_Component_C|GetEnableShatter (Variables|/Game/FirstPerson/Blueprints/BP_FirstPersonCharacter.BP_FirstPersonCharacter_C|GetBP_Weapon_Component _asbp_first_person_character))
    (CallFunction|ShatterCheck))
  (if (> (Variables|Default|GetHealth) 0.0)
    (Variables|Default|SetHealth (- (Variables|Default|GetHealth) Damage))
    (Variables|Default|SetisSeeingPlayer true)
    (CallFunction|FollowPlayer)
    (else
      (CallFunction|Death))))

(event EventTick
  (params (DeltaSeconds :type Float%20%28single-precision%29))
  ;[1 1 1] Update
  ;;[1 1 1] Health Bar
  (bind _aswp_enemy_health_bar (Utilities|Casting|CastToWP_EnemyHealthBar (UserInterface|GetWidget (Variables|Default|GetHealthBarWidget))))
  (Progress|SetPercent (Variables|/Game/UI/WP_EnemyHealthBar.WP_EnemyHealthBar_C|GetHealthBar _aswp_enemy_health_bar) (/ (Variables|Default|Gethealth) (Variables|Default|GetmaxHealth)))
  (Transformation|SetWorldRotation (Variables|Default|GetHealthBarWidget) (Math|Rotator|FindLookatRotation (Transformation|GetWorldLocation (Variables|Default|GetHealthBarWidget)) (Transformation|GetWorldLocation (Variables|/Script/Engine.PlayerCameraManager|GetTransformComponent (Game|GetPlayerCameraManager 0)))) false false)
  (Default|GetStacks _aswp_enemy_health_bar (Variables|Default|GetslowStacks))
  (Default|DisplayBurn _aswp_enemy_health_bar (Variables|Default|GetisBurning))
  (Default|DisplayBleed _aswp_enemy_health_bar (Variables|Default|GetisBleeding))
  (if (Variables|Default|GetisRoaming)
    (Variables|/Script/Engine.CharacterMovementComponent|SetMaxWalkSpeed (Variables|Character|GetCharacterMovement) (/ (Variables|Default|GetmaxMoveSpeed) 4.0))
    (else
      (if (Variables|Default|GetisBurning)
        (CallFunction|MoveSpeedBuff))
      (Variables|/Script/Engine.CharacterMovementComponent|SetMaxWalkSpeed (Variables|Character|GetCharacterMovement) (Variables|Default|GetcurrentMoveSpeed))))
  (if (<= (Variables|Default|Gethealth) 0.0)
    (CallFunction|Death)))

(event EventBeginPlay
  (bind _difficulty (Variables|Default|Getdifficulty))
  ;[1 1 1] Start
  (Variables|Default|SetmaxHealth (* (Variables|Default|GetmaxHealth) _difficulty))
  (Variables|Default|Setdamage (* (Variables|Default|Getdamage) _difficulty))
  (Variables|Default|Sethealth (Variables|Default|GetmaxHealth))
  (Variables|Default|SetcurrentMoveSpeed (Variables|Default|GetmaxMoveSpeed))
  (if (not (Variables|Default|GetisSeeingPlayer))
    (CallFunction|RandomRoam)))

(fn ConstructionScript
  (CallFunction|AlterDifficulty (Variables|Default|Getdifficulty))
  (CallFunction|AlterXPGiven (Variables|Default|GetxpGiven)))