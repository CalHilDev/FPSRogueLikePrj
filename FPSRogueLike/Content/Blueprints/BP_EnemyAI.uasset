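; Enemy character that roams random points, chases and melee-attacks the player on sight or when hurt, and grants XP on death.
; Bleed and burn tick damage through looping timers sharing one handle; chill stacks enable a shatter hit during burn.
; Tick turns the health bar to the camera and rewrites walk speed, overriding the burn boost and chill slow.
; Only AnyDamage checks for death, so status damage alone never kills.
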(event OnSeePawn(PawnSensing)
  (params (Pawn :type Pawn%20Object%20Reference))
  ;[1 1 1] Enable Chase State
  (Variables|Default|SetisSeeingPlayer true)
  (CallFunction|FollowPlayer))

(event Custom|FollowPlayer
  ;[1 1 1] Chase & Attack
  (Variables|Default|SetisRoaming false)
  (Variables|Default|SetcanAttack true)
  (if (Variables|Default|GetisSeeingPlayer)
    (AI|AIMoveTo self "0, 0, 0" (Game|GetPlayerCharacter 0) 5.0 false
      (:OnSuccess
        (if (Variables|Default|GetcanAttack)
          (Variables|Default|SetcanAttack false)
          (bind _returnvalue (Animation|PlayAnimMontage "/Game/Animations/EnemyAI/AM_EnemyAttack.AM_EnemyAttack" 1.0 "None"))
          (Game|Damage|ApplyDamage (Game|GetPlayerCharacter 0) (Variables|Default|Getdamage) 0 0)
          (Utilities|FlowControl|Delay _returnvalue))))
    (else
      (Variables|Default|SetisSeeingPlayer false))))

(event Custom|XPBuff
  ;[1 1 1] Increase XP
  (Variables|Default|SetxpGiven (* (Variables|Default|GetxpGiven) 1.1)))

(event Custom|BleedCheck
  (params (bleedCheck :type Boolean))
  ;[1 1 1] Bleeding
  (bind _output_get (Variables|Default|SetisBleeding bleedCheck))
  (if _output_get
    (CallFunction|Bleeding)))

(event Custom|SetBleedDamage
  (params (WeaponDamage :type Float%20%28double-precision%29))
  ;[1 1 1] Bleeding
  (Variables|Default|SetbleedDamage (* WeaponDamage 0.2)))

(event Custom|ApplyBleed
  (bind _bleeddamage (Variables|Default|GetbleedDamage))
  (bind _bleedduration (Variables|Default|GetbleedDuration))
  (bind _returnvalue (/ _bleeddamage _bleedduration))
  ;[1 1 1] Bleeding
  (Variables|Default|Sethealth (- (Variables|Default|Gethealth) _returnvalue))
  (Variables|Default|SetbleedDamageAccumulated (+ _returnvalue (Variables|Default|GetbleedDamageAccumulated)))
  (bind _output_get (Variables|Default|SetbleedDone (>= (Variables|Default|GetbleedDamageAccumulated) (Variables|Default|GetbleedDamage))))
  (if _output_get
    (Utilities|Time|ClearandInvalidateTimerbyHandle (Variables|Default|GetdamageTimer))
    (Variables|Default|SetisBleeding false)
    (Variables|Default|SetbleedDone false)
    (Variables|Default|SetbleedDamageAccumulated 0.0)))

(event Custom|Bleeding
  ;[1 1 1] Bleeding
  (bind _returnvalue (Utilities|Time|SetTimerbyEvent (delegate Custom|ApplyBleed) 1.0 true))
  (Variables|Default|SetdamageTimer _returnvalue))

(event Custom|ShatterCheck
  ;[1 1 1] Shatter Check
  (if (>= (Variables|Default|GetslowStacks) 5)
    (Variables|Default|SetcanShatter true)
    (if (<= (Variables|Default|GetslowStacks) 4)
      (Variables|Default|SetcanShatter false))))

(event Custom|SetShatterDamage
  (params (weaponDamage :type Float%20%28double-precision%29))
  ;[1 1 1] Shatter
  (Variables|Default|SetshatterDamage (* weaponDamage (Variables|Default|GetshatterMuiltiplier))))

(event Custom|BurnCheck
  (params (burnCheck :type Boolean))
  ;[1 1 1] Burning
  (bind _output_get (Variables|Default|SetisBurning burnCheck))
  (if _output_get
    (CallFunction|Burning)))

(event Custom|SetBurnDamage
  (params (WeaponDamage :type Float%20%28double-precision%29))
  ;[1 1 1] Burning
  (Variables|Default|SetburnDamage (* WeaponDamage 0.5)))

(event Custom|ApplyBurn
  (bind _burndamage (Variables|Default|GetburnDamage))
  (bind _burnduration (Variables|Default|GetburnDuration))
  (bind _returnvalue (/ _burndamage _burnduration))
  ;[1 1 1] Burning
  (CallFunction|MoveSpeedBuff)
  (if (Variables|Default|GetcanShatter)
    (CallFunction|Shatter))
  (Variables|Default|Sethealth (- (Variables|Default|Gethealth) _returnvalue))
  (Variables|Default|SetburnDamageAccumulated (+ _returnvalue (Variables|Default|GetburnDamageAccumulated)))
  (bind _output_get (Variables|Default|SetburnDone (>= (Variables|Default|GetburnDamageAccumulated) (Variables|Default|GetburnDamage))))
  (if _output_get
    (Utilities|Time|ClearandInvalidateTimerbyHandle (Variables|Default|GetdamageTimer))
    (Variables|Default|SetisBurning false)
    (Variables|Default|SetburnDone false)
    (Variables|Default|SetburnDamageAccumulated 0.0)))

(event Custom|Burning
  ;[1 1 1] Burning
  (bind _returnvalue (Utilities|Time|SetTimerbyEvent (delegate Custom|ApplyBurn) 1.0 true))
  (Variables|Default|SetdamageTimer _returnvalue))

(event Custom|MoveSpeedDebuff
  ;[1 1 1] Slow (from freezing)
  (if (not (Variables|Default|GetisBurning))
    (Math|Integer|IncrementInt (Variables|Default|GetslowStacks)
      (:%20%20
        (Variables|/Script/Engine.CharacterMovementComponent|SetMaxWalkSpeed (Variables|Character|GetCharacterMovement) (- (Variables|Default|GetmaxMoveSpeed) (* (Variables|Default|GetslowStacks) (Variables|Default|GetslowPotency))))
        (Utilities|FlowControl|Delay (Variables|Default|GetchillDuration)) ; Duration of MS decrease
        (Math|Integer|DecrementInt (Variables|Default|GetslowStacks))))))

(event Custom|MoveSpeedBuff
  ;[1 1 1] Speed Boost (from burning)
  (Variables|Default|SetslowStacks 0)
  (Variables|/Script/Engine.CharacterMovementComponent|SetMaxWalkSpeed (Variables|Character|GetCharacterMovement) (* (Variables|Default|GetmaxMoveSpeed) 1.3))
  (Utilities|FlowControl|Delay 5.0) ; Duration of MS increase
  (Variables|/Script/Engine.CharacterMovementComponent|SetMaxWalkSpeed (Variables|Character|GetCharacterMovement) (Variables|Default|GetmaxMoveSpeed)))

(event Custom|RandomRoam
  ;[1 1 1] Roaming
  (Variables|Default|SetisRoaming true)
  (AI|AIMoveTo self (.RandomLocation (AI|Navigation|GetRandomReachablePointinRadius (Transformation|GetActorLocation) 1e+03 0 0)) 0 5.0 false
    (:OnSuccess
      (Utilities|FlowControl|Delay 1.0)
      (CallFunction|RandomRoam))))

(event Custom|Shatter
  ;[1 1 1] Shatter
  (Variables|Default|SetslowStacks 0)
  (Variables|Default|Sethealth (- (Variables|Default|Gethealth) (Variables|Default|GetshatterDamage))))

(event Game|Damage|EventAnyDamage
  (params (Damage :type Float%20%28single-precision%29) (DamageType :type Damage%20Type%20Object%20Reference) (InstigatedBy :type Controller%20Object%20Reference) (DamageCauser :type Actor%20Object%20Reference))
  ;[1 1 1] Take Damage
  (if (> (Variables|Default|GetHealth) 0.0)
    (Variables|Default|SetHealth (- (Variables|Default|GetHealth) Damage))
    (Variables|Default|SetisSeeingPlayer true)
    (CallFunction|FollowPlayer)
    (else
      (Actor|DestroyActor)
      (bind _asbp_first_person_character (Utilities|Casting|CastToBP_FirstPersonCharacter (Game|GetPlayerCharacter 0)))
      (Default|AddXP _asbp_first_person_character (Variables|Default|GetxpGiven)))))

(event EventTick
  (params (DeltaSeconds :type Float%20%28single-precision%29))
  ;[1 1 1] Update
  (Utilities|FlowControl|Sequence
    (:then_0
      ;;[1 1 1] Health Bar
      (bind _aswp_enemy_health_bar (Utilities|Casting|CastToWP_EnemyHealthBar (UserInterface|GetWidget (Variables|Default|GetHealthBarWidget))))
      (Progress|SetPercent (Variables|/Game/UI/WP_EnemyHealthBar.WP_EnemyHealthBar_C|GetHealthBar _aswp_enemy_health_bar) (/ (Variables|Default|Gethealth) (Variables|Default|GetmaxHealth)))
      (Transformation|SetWorldRotation (Variables|Default|GetHealthBarWidget) (Math|Rotator|FindLookatRotation (Transformation|GetWorldLocation (Variables|Default|GetHealthBarWidget)) (Transformation|GetWorldLocation (Variables|/Script/Engine.PlayerCameraManager|GetTransformComponent (Game|GetPlayerCameraManager 0)))) false false))
    (:then_1
      ;;[1 1 1] Updates Enemy Move Speed
      (Variables|/Script/Engine.CharacterMovementComponent|SetMaxWalkSpeed (Variables|Character|GetCharacterMovement) (Variables|Default|GetcurrentMoveSpeed))
      ;;[1 1 1] Roaming Speed
      (if (Variables|Default|GetisRoaming)
        (Variables|Default|SetcurrentMoveSpeed (/ (Variables|Default|GetmaxMoveSpeed) 4.0))
        (if (Variables|Default|GetisSeeingPlayer)
          (Variables|Default|SetisRoaming false)
          (elif (not (Variables|Default|GetisRoaming))
            (CallFunction|RandomRoam)))
        (else
          (Variables|Default|SetcurrentMoveSpeed (Variables|Default|GetmaxMoveSpeed)))))))

(event EventBeginPlay
  ;[1 1 1] Start
  (Variables|Default|Sethealth (Variables|Default|GetmaxHealth))
  (Variables|Default|SetcurrentMoveSpeed (Variables|Default|GetmaxMoveSpeed))
  (if (not (Variables|Default|GetisSeeingPlayer))
    (CallFunction|RandomRoam)))

(fn ConstructionScript)