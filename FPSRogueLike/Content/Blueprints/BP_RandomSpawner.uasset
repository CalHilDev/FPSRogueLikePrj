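; BP_RandomSpawner periodically spawns BP_EnemyAI enemies at random reachable navmesh points around itself.
; A looping timer started on BeginPlay fires SpawnEnemy every SpawnTime seconds.
; Each spawn picks a point within a large radius, applies a random yaw, and passes in the EnemyDifficulty read from the player's BP_FirstPersonCharacter.
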(event Custom|SpawnEnemy
  (bind _asbp_first_person_character (Utilities|Casting|CastToBP_FirstPersonCharacter (Game|GetPlayerCharacter 0)))
  (Game|SpawnActorfromClass "/Game/Blueprints/BP_EnemyAI.BP_EnemyAI_C" (Math|Transform|MakeTransform (.RandomLocation (AI|Navigation|GetRandomReachablePointinRadius (Transformation|GetActorLocation) 1e+04 0 0)) (Math|Rotator|MakeRotator 0.0 0.0 (Math|Random|RandomFloatinRange 0.0 3.6e+02)) "1.000000,1.000000,1.000000") "Undefined" "MultiplyWithRoot" 0 (Variables|/Game/FirstPerson/Blueprints/BP_FirstPersonCharacter.BP_FirstPersonCharacter_C|GetEnemyDifficulty _asbp_first_person_character) 0))

(event EventBeginPlay
  (Utilities|Time|SetTimerbyEvent (delegate Custom|SpawnEnemy) (Variables|Default|GetSpawnTime) true))

(fn ConstructionScript)